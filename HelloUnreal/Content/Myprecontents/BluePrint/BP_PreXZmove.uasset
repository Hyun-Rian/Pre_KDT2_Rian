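; BP_PreXZmove is a Blueprint that moves its Sphere component back and forth along a diagonal in the relative XZ plane.
; Each Tick offsets X and Z equally by Speed scaled by delta time, with the IfMove flag choosing the direction.
; The flag flips once both axes pass the upper or lower bound, creating a continuous ping-pong without a timeline or clamping.
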(event EventTick
  (params (DeltaSeconds :type Float%20%28single-precision%29))
  (bind _speed (Variables|Default|Getspeed))
  (bind _speed_2 (Variables|Default|Getspeed))
  (bind _sphere (Variables|Default|GetSphere))
  (bind _sphere_2 (Variables|Default|GetSphere))
  (bind _returnvalue (* DeltaSeconds _speed_2))
  (bind _returnvalue_2 (* DeltaSeconds _speed))
  (bind _returnvalue_3 (* _returnvalue_2 -1.0))
  (if (Variables|Default|GetIfMove)
    ;[1 1 1] 위로
    (Transformation|AddRelativeLocation _sphere_2 (Math|Vector|MakeVector _returnvalue 0.0 _returnvalue) false false)
    ;[1 1 1] 반환점
    (if (>= (.x (Variables|/Script/Engine.SceneComponent|GetRelativeLocation _sphere_2)) 5e+02)
      (if (>= (.z (Variables|/Script/Engine.SceneComponent|GetRelativeLocation _sphere_2)) 5e+02)
        (Variables|Default|SetIfMove false)))
    (else
      ;[1 1 1] 아래로
      (Transformation|AddRelativeLocation _sphere (Math|Vector|MakeVector _returnvalue_3 0.0 _returnvalue_3) false false)
      ;[1 1 1] 반환점
      (if (<= (.x (Variables|/Script/Engine.SceneComponent|GetRelativeLocation _sphere)) 0.0)
        (if (<= (.z (Variables|/Script/Engine.SceneComponent|GetRelativeLocation _sphere)) 0.0)
          (Variables|Default|SetIfMove true))))))

(fn ConstructionScript)