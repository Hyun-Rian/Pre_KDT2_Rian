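; BP_MoveRhombus is a Blueprint that moves its static mesh diagonally in the relative XZ plane, with legs laid out as a rhombus.
; Each Tick switches on the MoveVector state to pick one of four diagonal directions, offsetting the mesh by Speed scaled by delta time.
; Each leg tests a relative X or Z limit and sets MoveVector on reaching it, though every assignment shows the same Vector_XY value.
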(event EventTick
  (params (DeltaSeconds :type Float%20%28single-precision%29))
  (bind _staticmesh (Variables|Default|GetStaticMesh))
  (bind _speed (Variables|Default|Getspeed))
  (bind _staticmesh_2 (Variables|Default|GetStaticMesh))
  (bind _staticmesh_3 (Variables|Default|GetStaticMesh))
  (bind _staticmesh_4 (Variables|Default|GetStaticMesh))
  (bind _returnvalue (* DeltaSeconds _speed))
  (bind _returnvalue_2 (* DeltaSeconds _speed))
  (bind _returnvalue_3 (* DeltaSeconds _speed))
  (bind _returnvalue_4 (* DeltaSeconds _speed))
  (bind _returnvalue_5 (* _returnvalue_3 -1.0))
  (switch Utilities|FlowControl|Switch|SwitchonEN_MoveXY_Type (Variables|Default|GetMoveVector)
    (:NewEnumerator0
      (Transformation|AddRelativeLocation _staticmesh_2 (Math|Vector|MakeVector _returnvalue 0.0 _returnvalue) false false)
      (if (>= (.x (Variables|/Script/Engine.SceneComponent|GetRelativeLocation _staticmesh_2)) 5e+02)
        (Variables|Default|SetMoveVector "NewEnumerator1")))
    (:NewEnumerator1
      (Transformation|AddRelativeLocation _staticmesh (Math|Vector|MakeVector (* _returnvalue_2 -1.0) 0.0 _returnvalue_2) false false)
      (if (<= (.x (Variables|/Script/Engine.SceneComponent|GetRelativeLocation _staticmesh)) 0.0)
        (Variables|Default|SetMoveVector "NewEnumerator2")))
    (:NewEnumerator2
      (Transformation|AddRelativeLocation _staticmesh_3 (Math|Vector|MakeVector _returnvalue_5 0.0 _returnvalue_5) false false)
      (if (<= (.x (Variables|/Script/Engine.SceneComponent|GetRelativeLocation _staticmesh_3)) -5e+02)
        (Variables|Default|SetMoveVector "NewEnumerator3")))
    (:NewEnumerator3
      (Transformation|AddRelativeLocation _staticmesh_4 (Math|Vector|MakeVector _returnvalue_4 0.0 (* _returnvalue_4 -1.0)) false false)
      (if (<= (.z (Variables|/Script/Engine.SceneComponent|GetRelativeLocation _staticmesh_4)) 0.0)
        (Variables|Default|SetMoveVector "NewEnumerator0")))))

(fn ConstructionScript)