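; BP_PreRotaion is a Blueprint that swings its Cube component back and forth around the roll axis.
; Every Tick it adds relative roll scaled by delta time and SpinAg, with the sign chosen by the Ifback flag.
; Ifback flips when the cube's relative roll reaches the 180 or 0 degree limit, intended as a ping-pong half-turn.
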(event EventTick
  (params (DeltaSeconds :type Float%20%28single-precision%29))
  (bind _cube (Variables|Default|GetCube))
  (bind _cube_2 (Variables|Default|GetCube))
  (if (Variables|Default|GetIfback)
    (Transformation|AddRelativeRotation _cube_2 (Math|Rotator|MakeRotator (* DeltaSeconds (Variables|Default|GetSpinAg)) 0.0 0.0) false false)
    (if (>= (.roll (Variables|/Script/Engine.SceneComponent|GetRelativeRotation _cube_2)) 1.8e+02)
      (Variables|Default|SetIfback false))
    (else
      (Transformation|AddRelativeRotation _cube (Math|Rotator|MakeRotator (* (* DeltaSeconds (Variables|Default|GetSpinAg)) -1.0) 0.0 0.0) false false)
      (if (<= (.roll (Variables|/Script/Engine.SceneComponent|GetRelativeRotation _cube)) 0.0)
        (Variables|Default|SetIfback true)))))

(fn ConstructionScript)