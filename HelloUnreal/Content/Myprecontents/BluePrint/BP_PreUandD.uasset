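; BP_PreUandD is an actor that moves its Sphere component up and down in a continuous vertical loop.
; Each Tick offsets the sphere's relative Z by Speed scaled by DeltaSeconds, so the motion is frame-rate independent.
; The IfMoveUD boolean sets the direction and flips when the sphere passes the fixed upper or lower turning point, without clamping the overshoot.
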(event EventTick
  (params (DeltaSeconds :type Float%20%28single-precision%29))
  (bind _sphere (Variables|Default|GetSphere))
  (bind _sphere_2 (Variables|Default|GetSphere))
  (if (Variables|Default|GetIfMoveU&D)
    ;[1 1 1] 위로
    (Transformation|AddRelativeLocation _sphere_2 (Math|Vector|MakeVector 0.0 0.0 (* DeltaSeconds (Variables|Default|Getspeed))) false false)
    ;[1 1 1] 반환점
    (if (>= (.z (Variables|/Script/Engine.SceneComponent|GetRelativeLocation _sphere_2)) 1e+03)
      (Variables|Default|SetIfMoveU&D false))
    (else
      ;[1 1 1] 아래로
      (Transformation|AddRelativeLocation _sphere (Math|Vector|MakeVector 0.0 0.0 (* (* DeltaSeconds (Variables|Default|Getspeed)) -1.0)) false false)
      ;[1 1 1] 반환점
      (if (<= (.z (Variables|/Script/Engine.SceneComponent|GetRelativeLocation _sphere)) 0.0)
        (Variables|Default|SetIfMoveU&D true)))))

(fn ConstructionScript)