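; BP_PreRandL is a Blueprint that moves its Sphere component back and forth along the relative X axis.
; Each Tick offsets the sphere by Speed scaled by delta time, in the direction set by the IfMoveRight flag.
; The flag flips when the sphere's relative X reaches either fixed turning point, the origin or 500 units, producing a continuous ping-pong motion.
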(event EventTick
  (params (DeltaSeconds :type Float%20%28single-precision%29))
  (bind _sphere (Variables|Default|GetSphere))
  (bind _sphere_2 (Variables|Default|GetSphere))
  (if (Variables|Default|GetIfMoveRight)
    ;[1 0.7707 0.1674] X축 우측이동
    (Transformation|AddRelativeLocation _sphere_2 (Math|Vector|MakeVector (* DeltaSeconds (Variables|Default|Getspeed)) 0.0 0.0) false false)
    ;[1 0.3672 0.9694] 반환점
    (if (>= (.x (Variables|/Script/Engine.SceneComponent|GetRelativeLocation _sphere_2)) 5e+02)
      (Variables|Default|SetIfMoveRight false))
    (else
      ;[0.3193 1 0.2779] x축 좌측이동
      (Transformation|AddRelativeLocation _sphere (Math|Vector|MakeVector (* (* DeltaSeconds (Variables|Default|Getspeed)) -1.0) 0.0 0.0) false false)
      ;[0.8963 0.3201 0.7964] 반환점
      (if (<= (.x (Variables|/Script/Engine.SceneComponent|GetRelativeLocation _sphere)) 0.0)
        (Variables|Default|SetIfMoveRight true)))))

(fn ConstructionScript)