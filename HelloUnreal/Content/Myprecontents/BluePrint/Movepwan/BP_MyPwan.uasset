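; BP_MyPwan is a pawn Blueprint that provides free movement on three axes and mouse look.
; MoveForward, MoveRight and MoveUp axis inputs offset the actor along its own direction vectors by a fixed step, without sweep collision or delta-time scaling.
; LookTurn and LookUp axis inputs feed controller yaw and pitch.
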(event Input|AxisEvents|InputAxisMoveForward
  (params (AxisValue :type Float%20%28single-precision%29))
  ;[0.3846 0.4252 1] 키보드 이동
  (Transformation|AddActorWorldOffset (* (Transformation|GetActorForwardVector) (* AxisValue 1e+01))))

(event Input|AxisEvents|InputAxisMoveRight
  (params (AxisValue :type Float%20%28single-precision%29))
  ;[0.3846 0.4252 1] 키보드 이동
  (Transformation|AddActorWorldOffset (* (Transformation|GetActorRightVector) (* AxisValue 1e+01))))

(event Input|AxisEvents|InputAxisLookUp
  (params (AxisValue :type Float%20%28single-precision%29))
  ;[0.3277 1 0.2491] 마우스 시점회전
  (Pawn|Input|AddControllerPitchInput AxisValue))

(event Input|AxisEvents|InputAxisLookTurn
  (params (AxisValue :type Float%20%28single-precision%29))
  ;[0.3277 1 0.2491] 마우스 시점회전
  (Pawn|Input|AddControllerYawInput AxisValue))

(event Input|AxisEvents|InputAxisMoveUp
  (params (AxisValue :type Float%20%28single-precision%29))
  ;[0.3846 0.4252 1] 키보드 이동
  (Transformation|AddActorWorldOffset (* (Transformation|GetActorUpVector) (* AxisValue 1e+01))))

(fn ConstructionScript)